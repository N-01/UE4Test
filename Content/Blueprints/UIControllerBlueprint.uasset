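; UI controller Blueprint that relays game events for time, notifications, end-game text and keys to the MainUI widget.
; Each event goes through a shared helper that casts the Widget component's user widget to MainUI and stops if the cast fails.
; Notifications clear themselves by sending empty text after a Delay, so a message shown during a pending delay is cleared on the earlier timer.
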(event EventBeginPlay)

(event Collision|EventActorBeginOverlap
  (params (OtherActor :type Actor%20Object%20Reference)))

(event EventSetTime
  (params (text :type String))
  (Default|SetTime (CallFunction|CasttoMainUI) text))

(event EventShowNotification
  (params (text :type String) (duration :type Float%20%28single-precision%29))
  (bind _newparam (CallFunction|CasttoMainUI))
  (Default|ShowNotification _newparam text)
  (Utilities|FlowControl|Delay duration)
  (Default|ShowNotification _newparam))

(event EventTick
  (params (DeltaSeconds :type Float%20%28single-precision%29)))

(event EventShowEndGame
  (params (text :type String))
  (Default|ShowEndGame (CallFunction|CasttoMainUI) text))

(event EventAddKey
  (params (key :type KeyColor%20Enum :default "Red"))
  (Default|AddKey (CallFunction|CasttoMainUI) key))

(event EventRemoveKey
  (params (key :type KeyColor%20Enum :default "Red"))
  (Default|RemoveKey (CallFunction|CasttoMainUI) key))

(fn ConstructionScript)

(fn CasttoMainUI
  (bind _asmain_ui (Utilities|Casting|CastToMainUI (UserInterface|GetUserWidgetObject (Variables|Default|GetWidget))))
  (return _asmain_ui))